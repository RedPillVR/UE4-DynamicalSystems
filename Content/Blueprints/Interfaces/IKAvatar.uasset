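; IKAvatar is a Blueprint interface for VR avatars, declaring functions with no logic of their own.
; Getters expose the avatar mesh, VR origin, camera, per-hand IK motion controller and Leap offset, several with a success flag.
; Other calls set the avatar's name and ID, calibrate height, teleport the avatar and notify it of left or right footsteps.
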(fn `CalibrateHeight`)

(fn `GetAvatarMesh`
  (returns (SkeletalMesh :type "SkeletalMeshComponent Object Reference"))
  (return null))

(fn `GetCamera`
  (returns (Camera :type "CameraComponent Object Reference") (Success :type Boolean))
  (return null false))

(fn `GetIKMotionController`
  (params (Hand :type "EControllerHand Enum" :default "Left"))
  (returns (IKMotionController :type "/DynamicalSystems/FullBodyIK/Blueprints/IK_MotionController Object Reference") (Success :type Boolean))
  (return null false))

(fn `GetLeapOffset`
  (returns (OffsetObject :type "SceneComponent Object Reference") (Success :type Boolean))
  (return null false))

(fn `GetVROrigin`
  (returns (Origin :type "SceneComponent Object Reference"))
  (return null))

(fn `Notify_Footstep`
  (params (Left :type Boolean) (On :type Boolean))
  (returns (Success :type Boolean))
  (return false))

(fn `SetAvatar`
  (params (Id :type Integer))
  (returns (Success :type Boolean))
  (return false))

(fn `SetName`
  (params (NewName :type Name))
  (returns (Success :type Boolean))
  (return false))

(fn `TeleportAvatar`
  (params (Position :type "Transform Structure")))