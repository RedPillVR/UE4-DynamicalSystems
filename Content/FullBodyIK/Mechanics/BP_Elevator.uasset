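; BP_Elevator is an actor that moves a Cube component back and forth between its Start and End transforms, acting as an automatic elevator.
; Each Tick, game time since creation, scaled by MoveSpeed and FlipSpeed and wrapped modulo 2, selects End or Start as the target.
; TInterpTo eases the cube toward that target at MoveSpeed, without sweeping, so MoveSpeed affects both easing and flip timing.
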(event `self.ReceiveTick`
  (params (DeltaSeconds :type "Float (single-precision)"))
  (bind _returnvalue (`SceneComponent.K2_GetComponentToWorld` (`self.Cube`)))
  (if (< (mod (* (`self.GetGameTimeSinceCreation`) (* (`self.MoveSpeed`) (`self.FlipSpeed`))) 2.0) 1.0)
    (`SceneComponent.K2_SetWorldTransform` (`self.Cube`) (`KismetMathLibrary.TInterpTo` _returnvalue (`SceneComponent.K2_GetComponentToWorld` (`self.End`)) DeltaSeconds (`self.MoveSpeed`)) false false)
    (else
      (`SceneComponent.K2_SetWorldTransform` (`self.Cube`) (`KismetMathLibrary.TInterpTo` _returnvalue (`SceneComponent.K2_GetComponentToWorld` (`self.Start`)) DeltaSeconds (`self.MoveSpeed`)) false false))))

(fn `UserConstructionScript`)