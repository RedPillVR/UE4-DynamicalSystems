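; VR pawn for a networked full-body IK avatar, loaded from a data table, with HMD, motion controllers and Leap hand visibility.
; Each tick the local pawn applies traced gravity and writes mesh-relative tracking transforms to AvatarState on the PlayerState; remote pawns apply that state.
; BeginPlay spawns a center-of-mass actor and a PID follower.
; Bezier center-of-mass and hand/head offset functions are defined but not called here.
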(event `self.ReceiveBeginPlay`
  (bind _leap (`self.Leap`))
  (`|ExecutionSequence`
    (:`then_0`
      (`self.SetupTransforms`)
      ;[0 0 0] Determine HMD Type
      (switch `name` (`HeadMountedDisplayFunctionLibrary.GetHMDDeviceName`)
        (:`OculusHMD`
          (set `self.DeviceList` "NewEnumerator0"))
        (:`SteamVR`
          (set `self.DeviceList` "NewEnumerator1"))))
    (:`then_1`
      (add `LeapComponent.OnLeftHandVisibilityChanged` _leap (delegate `OnLeftHandVisibilityChanged_Event_0`))
      (add `LeapComponent.OnRightHandVisibilityChanged` _leap (delegate `OnRightHandVisibilityChanged_Event_0`)))))

(event `OnLeftHandVisibilityChanged_Event_0`
  (params (bIsVisible :type Boolean))
  (set `/DynamicalSystems/State/AvatarState.LeftIsVisible` bIsVisible (`self.GetState`)))

(event `OnRightHandVisibilityChanged_Event_0`
  (params (bIsVisible :type Boolean))
  (set `/DynamicalSystems/State/AvatarState.RightIsVisible` bIsVisible (`self.GetState`)))

(event `self.ReceiveTick`
  (params (DeltaSeconds :type "Float (single-precision)"))
  (`|ExecutionSequence`
    (:`then_0`
      (`self.ApplyGravity` DeltaSeconds)
      (`SceneComponent.K2_SetRelativeLocation` (`self.AvatarMesh`) (* (.location (`SceneComponent.GetRelativeTransform` (`self.HMDCamera`))) (1.0 1.0 0.0)) false false))
    (:`then_1`
      (`self.SendNetwork`))
    (:`then_2`
      (`self.ReceiveNetwork`))
    (:`then_3`
      (`self.DebugTransforms`))))

(event `InputAxis|RiftMotionControllerThumbLeft_X`
  (params (AxisValue :type "Float (single-precision)")))

(event `InputAxis|RiftMotionControllerThumbLeft_Y`
  (params (AxisValue :type "Float (single-precision)")))

(event `InputAxis|RiftMotionControllerThumbRight_X`
  (params (AxisValue :type "Float (single-precision)")))

(event `InputAxis|RiftMotionControllerThumbRight_Y`
  (params (AxisValue :type "Float (single-precision)")))

(event `InputAxis|ViveMotionControllerThumbLeft_X`
  (params (AxisValue :type "Float (single-precision)")))

(event `InputAxis|ViveMotionControllerThumbLeft_Y`
  (params (AxisValue :type "Float (single-precision)")))

(event `InputAxis|ViveMotionControllerThumbRight_X`
  (params (AxisValue :type "Float (single-precision)")))

(event `InputAxis|ViveMotionControllerThumbRight_Y`
  (params (AxisValue :type "Float (single-precision)")))

(fn `ApplyGravity`
  (params (DeltaTime :type "Float (double-precision)"))
  (bind _origin (`self.Origin`))
  (bind _returnvalue (* (`self.GravityMultiplier`) (`self.GravityStrength`) DeltaTime))
  (if (`self.IsLocallyControlled`)
    (bind (_outhit _returnvalue_2) (`self.TraceForGround` 80.0))
    (if _returnvalue_2
      (bind (_bblockinghit _binitialoverlap _time _distance _location) (`GameplayStatics.BreakHitResult` _outhit))
      (if (> _distance _returnvalue)
        _
        (else
          _))
      (`SceneComponent.K2_SetWorldLocation` _origin _location false false)
      (else
        (`SceneComponent.K2_AddWorldOffset` _origin (* (0.0 0.0 -1.0) _returnvalue) false false)))))

(fn `ApplyTransforms`
  (bind (_returnvalue_location _returnvalue_rotation) (`KismetMathLibrary.BreakTransform` (`self.GetTransform` (`ChildActorComponent.ChildActor` (`self.ChildHMD`)))))
  (bind _returnvalue (`KismetMathLibrary.ComposeTransforms` (`self.HeadOffset`) (`KismetMathLibrary.MakeTransform` _returnvalue_location _returnvalue_rotation)))
  (`|ExecutionSequence`
    (:`then_0`
      (set `self.HandRAnim` (`KismetMathLibrary.ComposeTransforms` (`self.HandOffsetR`) (`self.GetTransform` (`ChildActorComponent.ChildActor` (`self.ChildMotionControllerR`))))))
    (:`then_1`
      (set `self.HandLAnim` (`KismetMathLibrary.ComposeTransforms` (`self.HandOffsetL`) (`self.GetTransform` (`ChildActorComponent.ChildActor` (`self.ChildMotionControllerL`))))))
    (:`then_2`
      (set `self.HeadAnim` (`KismetMathLibrary.MakeTransform` (.location _returnvalue) (`KismetMathLibrary.MakeRotator` (.roll (.rotation _returnvalue)) (`KismetMathLibrary.FClamp` (.pitch (.rotation _returnvalue)) 80.0 110.0) (.yaw (.rotation _returnvalue))) (.scale _returnvalue))))
    (:`then_4`
      (return))))

(fn `ClampUpTransform`
  (params (In :type "Transform Structure"))
  (returns (Out :type "Transform Structure"))
  (locals (Transform :type Boolean))
  (bind _rotation (.rotation In))
  (bind _returnvalue (`KismetMathLibrary.GetUpVector` _rotation))
  (bind _returnvalue_2 (`KismetMathLibrary.MapRangeUnclamped` (`KismetMathLibrary.Dot_VectorVector` _returnvalue (0.0 0.0 -1.0)) -1.0 1.0 0.0 1.0))
  (bind _returnvalue_3 (- 1.0 _returnvalue_2))
  (return (`KismetMathLibrary.MakeTransform` (.location In) (`KismetMathLibrary.MakeRotFromXY` (+ (* _returnvalue _returnvalue_2) (* (`KismetMathLibrary.GetForwardVector` _rotation) _returnvalue_3)) (* (`KismetMathLibrary.GetRightVector` _rotation) _returnvalue_3)) (.scale In))))

(fn `DebugTransforms`
  (bind (_asavatar_state _bsuccess) (`self.GetState`))
  (bind _avatarmesh (`self.AvatarMesh`))
  (bind _returnvalue (`SceneComponent.K2_GetComponentLocation` _avatarmesh))
  (bind _returnvalue_2 (`SceneComponent.K2_GetComponentToWorld` (`self.Origin`)))
  (if (`self.Debug`)
    (if _bsuccess
      (`|ExecutionSequence`
        (:`then_0`
          (`KismetSystemLibrary.DrawDebugArrow` _returnvalue (+ _returnvalue (* (`SceneComponent.GetForwardVector` _avatarmesh) 20.0)) 20.0 (struct :`G` 0.054582 :`B` 1.0 :`A` 1.0) 0.0 20.0))
        (:`then_1`
          (`|ExecutionSequence`
            (:`then_0`
              (`KismetSystemLibrary.DrawDebugFrustum` (`KismetMathLibrary.ComposeTransforms` (`/DynamicalSystems/State/AvatarState.Avatar_CenterOfMass` _asavatar_state) (`KismetMathLibrary.MakeTransform` (0.0 0.0 0.0) (struct :`Pitch` 90.0 :`Yaw` 90.0))) (struct :`G` 0.842055 :`B` 1.0 :`A` 1.0) 0.0 20.0)
              (`KismetSystemLibrary.DrawDebugFrustum` (`KismetMathLibrary.ComposeTransforms` (`SceneComponent.K2_GetComponentToWorld` (`/DynamicalSystems/FullBodyIK/Blueprints/IK_Transform.DefaultSceneRoot` (`self.CenterOfMass`))) (`KismetMathLibrary.MakeTransform` (0.0 0.0 0.0) (struct :`Yaw` -90.0))) (struct :`R` 1.0 :`G` 0.517713 :`A` 1.0) 0.0 20.0))
            (:`then_1`
              (`KismetSystemLibrary.DrawDebugFrustum` (`/DynamicalSystems/State/AvatarState.Avatar_Head` _asavatar_state) (struct :`R` 1.0 :`B` 0.784527 :`A` 1.0) 0.0 20.0))
            (:`then_2`
              (`KismetSystemLibrary.DrawDebugFrustum` (`KismetMathLibrary.ComposeTransforms` (`/DynamicalSystems/State/AvatarState.Avatar_LHand` _asavatar_state) _returnvalue_2) (struct :`G` 0.734626 :`B` 1.0 :`A` 1.0) 0.0 20.0))
            (:`then_3`
              (`KismetSystemLibrary.DrawDebugFrustum` (`KismetMathLibrary.ComposeTransforms` (`/DynamicalSystems/State/AvatarState.Avatar_RHand` _asavatar_state) _returnvalue_2) (struct :`R` 1.0 :`G` 0.057883 :`A` 1.0) 0.0 20.0))))))))

(fn `GetState`
  (returns (`AsAvatar State` :type "/DynamicalSystems/State/AvatarState Object Reference") (bSuccess :type Boolean))
  (bind (_asavatar_state _bsuccess) (cast `/DynamicalSystems/State/AvatarState` (`self.PlayerState`) :!pure true))
  (return _asavatar_state _bsuccess))

(fn `ReceiveNetwork`
  (bind (_asavatar_state _bsuccess) (`self.GetState`))
  (if (not (and (`self.IsLocallyControlled`) _bsuccess))
    (`|ExecutionSequence`
      (:`then_0`
        (`/DynamicalSystems/State/AvatarState.SetObjectToAvatar` _asavatar_state (`self.MotionController_L`) (`self.MotionController_R`) (`self.HMDCamera`) (`self.ChildHMD`) false 0.0 (`self.Origin`))))))

(fn `ScaleForHeight`
  (params (B :type "Float (double-precision)"))
  (returns (Z :type "Float (double-precision)"))
  (bind _asavatar_state (`self.GetState`))
  (bind _avatar_measureheight (`/DynamicalSystems/State/AvatarState.Avatar_MeasureHeight` _asavatar_state))
  (bind _returnvalue (/ B _avatar_measureheight))
  (bind (_avatar_measureheight_2 _avatar_hmdoffset _avatar_mcl_offset _avatar_mcr_offset) (`/DynamicalSystems/State/AvatarState.FindOffsets` _asavatar_state (`self.AvatarMesh`)))
  (`KismetSystemLibrary.PrintText` (`|FormatText` "Floor{ f} \nav {a} \nmulti {m } \n \nMeasurements \nh {h} \nho {ho} \nmcl {mcl} \nmcr {mcr}" B _avatar_measureheight _returnvalue _avatar_measureheight_2 (`KismetTextLibrary.Conv_TransformToText` _avatar_hmdoffset) (`KismetTextLibrary.Conv_TransformToText` _avatar_mcl_offset) (`KismetTextLibrary.Conv_TransformToText` _avatar_mcr_offset)))
  (`SceneComponent.SetWorldScale3D` (`self.AvatarMesh`) (`KismetMathLibrary.Conv_DoubleToVector` _returnvalue))
  (bind _output_get (set `/DynamicalSystems/State/AvatarState.AvatarScale` _returnvalue (`self.GetState`)))
  (return _output_get))

(fn `SendNetwork`
  (bind (_asavatar_state _bsuccess) (`self.GetState`))
  (bind _returnvalue (`SceneComponent.K2_GetComponentToWorld` (`self.AvatarMesh`)))
  (if (and (`self.IsLocallyControlled`) _bsuccess)
    (`|ExecutionSequence`
      (:`then_0`
        (`/DynamicalSystems/State/AvatarState.SetIKTransform` _asavatar_state _returnvalue "NewEnumerator0"))
      (:`then_1`
        (`/DynamicalSystems/State/AvatarState.SetIKTransform` _asavatar_state (`KismetMathLibrary.ConvertTransformToRelative` _returnvalue (`SceneComponent.K2_GetComponentToWorld` (`self.HMDCamera`))) "NewEnumerator1"))
      (:`then_2`
        (`/DynamicalSystems/State/AvatarState.SetIKTransform` _asavatar_state (`KismetMathLibrary.ConvertTransformToRelative` _returnvalue (`SceneComponent.K2_GetComponentToWorld` (`self.MotionController_L`))) "NewEnumerator2"))
      (:`then_3`
        (`/DynamicalSystems/State/AvatarState.SetIKTransform` _asavatar_state (`KismetMathLibrary.ConvertTransformToRelative` _returnvalue (`SceneComponent.K2_GetComponentToWorld` (`self.MotionController_R`))) "NewEnumerator3"))
      (:`then_4`
        (`/DynamicalSystems/State/AvatarState.SetIK_Dimensions` _asavatar_state (`self.Floor`) "NewEnumerator1"))
      (:`then_5`
        (`/DynamicalSystems/State/AvatarState.SetIK_Dimensions` _asavatar_state (`self.Height`) "NewEnumerator0")))))

(fn `SetAvatar`
  (bind _asavatar_state (`self.GetState`))
  (bind _data (`/DynamicalSystems/FullBodyIK/Blueprints/IK_Utilities.GetAvatarFromTable` (`self.CurrentAvatarID`) (`self.AvatarTable`) (`self.LoadedAvatarTable`)))
  (`/DynamicalSystems/FullBodyIK/Blueprints/IK_Utilities.SetAvatar` _data (`self.AvatarMesh`))
  (`/Engine/EditorBlueprintResources/StandardMacros.IsValid` _asavatar_state
    (:`Is Valid`
      (`/DynamicalSystems/State/AvatarState.FindOffsets` _asavatar_state (`self.AvatarMesh`))
      (`KismetSystemLibrary.PrintText` (`|FormatText` "height: {j}" (`/DynamicalSystems/State/AvatarState.Avatar_MeasureHeight` _asavatar_state))))))

(fn `SetHeight`)

(fn `SetupTransforms`
  (bind _returnvalue (`SceneComponent.K2_GetComponentToWorld` (`self.MAssCenter`)))
  (`|ExecutionSequence`
    (:`then_1`
      (bind _returnvalue_2 (`|SpawnActorFromClass` "/DynamicalSystems/FullBodyIK/Blueprints/IK_Transform.IK_Transform_C" _returnvalue "AlwaysSpawn" "OverrideRootScale" self null))
      (bind _output_get (set `self.CenterOfMass` _returnvalue_2))
      (`PrimitiveComponent.SetMaterial` (`/DynamicalSystems/FullBodyIK/Blueprints/IK_Transform.Center` _output_get) 0 "/DynamicalSystems/FullBodyIK/Materials/MI_CenterOfMass.MI_CenterOfMass"))
    (:`then_2`
      (bind _returnvalue_3 (`|SpawnActorFromClass` "/DynamicalSystems/FullBodyIK/Blueprints/IK_Transform.IK_Transform_C" _returnvalue "AlwaysSpawn" "OverrideRootScale" self null))
      (`|ExecutionSequence`
        (:`then_0`
          (`PrimitiveComponent.SetMaterial` (`/DynamicalSystems/FullBodyIK/Blueprints/IK_Transform.Center` _returnvalue_3) 0 "/DynamicalSystems/FullBodyIK/Materials/MI_IMU.MI_IMU"))
        (:`then_1`
          (bind _returnvalue_4 (`AddComponent|NODE_AddTransformController-0` :`self` _returnvalue_3))
          (bind _output_get_2 (set `self.BodyIMU` _returnvalue_4))
          (`|ExecutionSequence`
            (:`then_0`
              (set `TransformController.LocationKp` (10.0 10.0 10.0) _output_get_2))
            (:`then_1`
              (set `TransformController.LocationKi` (0.0 0.0 0.0) _output_get_2))
            (:`then_2`
              (set `TransformController.LocationKd` (0.0 0.0 0.0) _output_get_2))
            (:`then_6`
              (set `TransformController.Target` (`self.CenterOfMass`) _output_get_2))))))))

(fn `TraceForGround`
  (params (TraceDistance :type "Float (double-precision)"))
  (returns (OutHit :type "HitResult Structure") (ReturnValue :type Boolean))
  (bind _returnvalue (`SceneComponent.K2_GetComponentLocation` (`self.Origin`)))
  (bind (_outhit _returnvalue_2) (`KismetSystemLibrary.LineTraceSingle` :`Start` (+ _returnvalue (* (0.0 0.0 1.0) (/ TraceDistance 2.0))) :`End` (+ _returnvalue (* _returnvalue (* (0.0 0.0 -1.0) TraceDistance))) :`TraceChannel` "TraceTypeQuery3" :`DrawDebugType` "ForOneFrame"))
  (return _outhit _returnvalue_2))

(fn `UpdateCenterOfMass`
  (params (delta :type "Float (double-precision)"))
  (bind (_returnvalue_x _returnvalue_y _returnvalue_z) (`KismetMathLibrary.BreakVector` (`SceneComponent.K2_GetComponentLocation` (`self.Origin`))))
  (bind (_returnvalue_x_2 _returnvalue_y_2) (`KismetMathLibrary.BreakVector` (`SceneComponent.K2_GetComponentLocation` (`/DynamicalSystems/FullBodyIK/Blueprints/IK_Transform.DefaultSceneRoot` (`self.CenterOfMass`)))))
  (`SceneComponent.K2_SetWorldLocation` (`self.Origin`) (`KismetMathLibrary.VInterpTo` (`SceneComponent.K2_GetComponentLocation` (`self.Origin`)) (`KismetMathLibrary.MakeVector` _returnvalue_x_2 _returnvalue_y_2 _returnvalue_z) delta 5.0) false false)
  (`SceneComponent.K2_SetWorldRotation` (`self.DefaultSceneRoot`) (`SceneComponent.K2_GetComponentRotation` (`self.Origin`)) false false))

(fn `UpdateTransforms`
  (bind (_asavatar_state _bsuccess) (`self.GetState`))
  (bind _returnvalue_location (`KismetMathLibrary.BreakTransform` (`SceneComponent.K2_GetComponentToWorld` (`self.ChildHMD`))))
  (bind _location (.location (`SceneComponent.K2_GetComponentToWorld` (`self.ChildHMD`))))
  (bind _returnvalue (`KismetMathLibrary.MakeTransform` (+ _location (`KismetMathLibrary.ClampVectorSize` (- (.location (`SceneComponent.K2_GetComponentToWorld` (`self.DefaultSceneRoot`))) _location) 0.0 (`self.Height`))) (.rotation (`SceneComponent.K2_GetComponentToWorld` (`self.DefaultSceneRoot`))) (.scale (`SceneComponent.K2_GetComponentToWorld` (`self.DefaultSceneRoot`)))))
  (bind _location_2 (.location _returnvalue))
  (bind _returnvalue_2 (/ (`KismetMathLibrary.VSize` (- _returnvalue_location _location_2)) (`self.Height`)))
  (`SceneComponent.K2_SetWorldLocation` (`/DynamicalSystems/FullBodyIK/Blueprints/IK_Transform.DefaultSceneRoot` (`self.CenterOfMass`)) (`DynamicalUtil.CubicBezier` 0.45 _returnvalue_location (`KismetMathLibrary.TransformLocation` (`self.ClampUpTransform` (`SceneComponent.K2_GetComponentToWorld` (`self.ChildHMD`))) (* (`KismetMathLibrary.MakeVector` (`KismetMathLibrary.MapRangeClamped` _returnvalue_2 1.0 0.0 -20.0 -100.0) 0.0 (`KismetMathLibrary.MapRangeClamped` _returnvalue_2 1.0 0.0 -50.0 50.0)) _returnvalue_2)) (`KismetMathLibrary.TransformLocation` _returnvalue (* (`KismetMathLibrary.MakeVector` 0.0 (`KismetMathLibrary.MapRangeClamped` _returnvalue_2 1.0 0.0 -1.0 -50.0) (`KismetMathLibrary.MapRangeClamped` _returnvalue_2 1.0 0.0 50.0 -50.0)) 1.0)) _location_2) false false)
  (if _bsuccess
    (set `/DynamicalSystems/State/AvatarState.Avatar_HMDVelocity` (`TransformController.LocationControl` (`self.BodyIMU`)) _asavatar_state)))

(fn `UserConstructionScript`
  (bind _avatarmesh (`self.AvatarMesh`))
  (`parent.UserConstructionScript`)
  (`self.SetAvatar`)
  (`SceneComponent.K2_AttachToComponent` (`self.ChildMotionControllerL`) (`self.MotionController_L`) "None" "SnapToTarget" "SnapToTarget" "SnapToTarget" true)
  (`SceneComponent.K2_AttachToComponent` (`self.ChildMotionControllerR`) (`self.MotionController_R`) "None" "SnapToTarget" "SnapToTarget" "SnapToTarget" true)
  (`SceneComponent.K2_AttachToComponent` (`self.ChildHMD`) (`self.HMDCamera`) "None" "SnapToTarget" "SnapToTarget" "SnapToTarget" true)
  (set `self.OriginalHeight` (- (`SceneComponent.GetSocketLocation` _avatarmesh "HMD") (`SceneComponent.GetSocketLocation` _avatarmesh "Floor"))))