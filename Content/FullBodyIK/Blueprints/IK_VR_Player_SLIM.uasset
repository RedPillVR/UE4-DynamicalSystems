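; Slim VR player controller for full-body IK that feeds the pawn's tracked HMD and motion controllers into the AvatarState player state.
; Validation finds the pawn, spawns an IK_Camera and caches its controllers.
; Tick then pushes IK transforms, floor and height with debug shapes, runs locomotion with zero delta time, and updates the avatar from state.
; Floor-snapping and grip-latch climbing events exist, but their calls are disconnected.
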(event `self.ReceiveBeginPlay`
  (`|ExecutionSequence`
    (:`then_0`
      (`HeadMountedDisplayFunctionLibrary.SetTrackingOrigin` "Floor"))
    (:`then_1`
      (set `/DynamicalSystems/State/AvatarState.Controller` self (`self.GetState`)))))

(event `Spawned`
  (params (Camera :type "/DynamicalSystems/FullBodyIK/Blueprints/IK_Camera Object Reference") (Pawn :type "/DynamicalSystems/FullBodyIK/Blueprints/IK_Pawn Object Reference"))
  (set `self.IK_Pawn` Pawn)
  (set `self.IK_Camera` Camera))

(event `self.ReceiveTick`
  (params (DeltaSeconds :type "Float (single-precision)"))
  (if (`self.Valid`)
    (`|ExecutionSequence`
      (:`then_0`
        (`|ExecutionSequence`
          (:`then_2`
            (`self.SetNetworkTransforms`))
          (:`then_3`
            (`self.MotionLocomotion` 0.0))))
      (:`then_1`
        (`self.UpdateFromState` DeltaSeconds)))
    (else
      (bind _isvalid (`self.Validation`))
      (set `self.Valid` _isvalid))))

(event `InputAction|CalibrateHeight`
  (params (Key :type "Key Structure"))
  ;[0 0 0] Calibrate Height on Controller until keyboard shows up in builds correctly.
  (:`Pressed`
    (`self.CalibrateHeight`)))

(event `self.FloorNav`
  (params (DeltaTime :type "Float (single-precision)"))
  (bind _ik_camera (`self.IK_Camera`))
  (bind _ik_pawn (`self.IK_Pawn`))
  (bind _defaultsceneroot (`/DynamicalSystems/FullBodyIK/Blueprints/IK_Camera.DefaultSceneRoot` (`self.IK_Camera`)))
  (bind _returnvalue (`SceneComponent.K2_GetComponentLocation` (`/DynamicalSystems/FullBodyIK/Blueprints/IK_Pawn.DefaultSceneRoot` (`self.IK_Pawn`))))
  (bind (_returnvalue_x _returnvalue_y _returnvalue_z) (`KismetMathLibrary.BreakVector` (`SceneComponent.K2_GetComponentLocation` (`/DynamicalSystems/FullBodyIK/Blueprints/IK_Camera.DefaultSceneRoot` _ik_camera))))
  (bind (_returnvalue_x_2 _returnvalue_y_2 _returnvalue_z_2) (`KismetMathLibrary.BreakVector` (`SceneComponent.K2_GetComponentLocation` (`/DynamicalSystems/FullBodyIK/Blueprints/IK_Pawn.DefaultSceneRoot` (`self.IK_Pawn`)))))
  (bind (_returnvalue_x_3 _returnvalue_y_3) (`KismetMathLibrary.BreakVector` (`SceneComponent.K2_GetComponentLocation` _defaultsceneroot)))
  (bind _x (.x (`SceneComponent.K2_GetComponentLocation` (`/DynamicalSystems/FullBodyIK/Blueprints/IK_Pawn.DefaultSceneRoot` _ik_pawn))))
  (bind _y (.y (`SceneComponent.K2_GetComponentLocation` (`/DynamicalSystems/FullBodyIK/Blueprints/IK_Pawn.DefaultSceneRoot` _ik_pawn))))
  (bind _z (.z (`SceneComponent.K2_GetComponentLocation` (`/DynamicalSystems/FullBodyIK/Blueprints/IK_Pawn.DefaultSceneRoot` _ik_pawn))))
  (if (and (`KismetSystemLibrary.IsValid` _ik_camera) (`KismetSystemLibrary.IsValid` _ik_pawn))
    (set `self.HeadOffset_0` (- _returnvalue_z _z))
    (bind (_outhit _returnvalue_2) (`KismetSystemLibrary.LineTraceSingleForObjects` (`KismetMathLibrary.MakeVector` _x _y (+ _z 100.0)) (`KismetMathLibrary.MakeVector` _x _y (+ _z -20000.0)) (`|MakeArray` "ObjectTypeQuery1" "ObjectTypeQuery14" "ObjectTypeQuery10" :!type "EObjectTypeQuery Enum") false (`|MakeArray` (`self.IK_Pawn`) :!type "Actor Object Reference")))
    (if _returnvalue_2
      (bind (_bblockinghit _binitialoverlap _time _distance _location _impactpoint _normal) (`GameplayStatics.BreakHitResult` _outhit))
      (`SceneComponent.K2_SetWorldLocation` (`/DynamicalSystems/FullBodyIK/Blueprints/IK_Pawn.DefaultSceneRoot` (`self.IK_Pawn`)) (`KismetMathLibrary.VInterpTo` _returnvalue _location DeltaTime (`KismetMathLibrary.MapRangeClamped` (.z (- _location _returnvalue)) 50.0 -50.0 (* 1.0 20.0) (* (`self.Gravity`) 1.0))) false false)
      (bind _output_get (set `/DynamicalSystems/FullBodyIK/Blueprints/IK_Pawn.Floor` (.z _location) (`self.IK_Pawn`)))
      (`SceneComponent.K2_SetWorldLocation` _defaultsceneroot (`KismetMathLibrary.MakeVector` _returnvalue_x_3 _returnvalue_y_3 (+ (`self.HeadOffset_0`) _returnvalue_z_2)) false false))))

(event `self.Latch`
  (params (DeltaTime :type "Float (single-precision)"))
  (bind _gravitycurve (`self.GravityCurve`))
  (bind _returnvalue (`SceneComponent.K2_GetComponentLocation` (`/DynamicalSystems/FullBodyIK/Blueprints/IK_MotionController.OVSphere` (`self.IK_MotionControllerR`))))
  (bind _returnvalue_2 (`SceneComponent.K2_GetComponentLocation` (`/DynamicalSystems/FullBodyIK/Blueprints/IK_MotionController.OVSphere` (`self.IK_MotionControllerL`))))
  (if (and (`KismetSystemLibrary.IsValid` (`self.IK_MotionControllerL`)) (`KismetSystemLibrary.IsValid` (`self.IK_Camera`)) (`KismetSystemLibrary.IsValid` (`self.IK_Pawn`)))
    (`|ExecutionSequence`
      (:`then_0`
        (set `self.GripLockedOffsetR` (`KismetMathLibrary.VLerp` (`self.GripLockedOffsetR`) (0.0 0.0 0.0) (* DeltaTime 0.5))))
      (:`then_1`
        (set `self.GripLockedOffsetL` (`KismetMathLibrary.VLerp` (`self.GripLockedOffsetL`) (0.0 0.0 0.0) (* DeltaTime 0.5))))
      (:`then_2`
        (if (and (> (`self.GetInputAxisValue`) 0.5) (`/DynamicalSystems/FullBodyIK/Blueprints/IK_MotionController.IsOverlapping` (`self.IK_MotionControllerL`)))
          (if (not (`self.GripLockedL`))
            (set `self.GripLockedLocationL` _returnvalue_2)
            (set `self.GripLockedL` true)
            (set `self.GripLockedOffsetL` (0.0 0.0 0.0))
            (else
              (set `self.GripLockedOffsetL` (- (`self.GripLockedLocationL`) _returnvalue_2))))
          (elif (`self.GripLockedL`)
            (set `self.GripLockedL` false))))
      (:`then_3`
        (if (and (> (`self.GetInputAxisValue`) 0.5) (`/DynamicalSystems/FullBodyIK/Blueprints/IK_MotionController.IsOverlapping` (`self.IK_MotionControllerR`)))
          (if (not (`self.GripLockedR`))
            (set `self.GripLockedLocationR` _returnvalue)
            (set `self.GripLockedR` true)
            (set `self.GripLockedOffsetR` (0.0 0.0 0.0))
            (else
              (set `self.GripLockedOffsetR` (- (`self.GripLockedLocationR`) _returnvalue))))
          (elif (`self.GripLockedR`)
            (set `self.GripLockedR` false))))
      (:`then_4`
        (set `self.Gravity` (`KismetMathLibrary.Lerp` (`self.Gravity`) (`self.DefaultGravity`) (* DeltaTime 0.5))))
      (:`then_5`
        (`/Engine/EditorBlueprintResources/StandardMacros.IsValid` _gravitycurve
          (:`Is Valid`
            (bind _output_get (set `self.DefaultGravity` (- 1.0 (`CurveFloat.GetFloatValue` (`/DynamicalSystems/Blueprints/BP_GravityCurve.GravityCurve` (`self.GravityCurve`)) (/ (`KismetMathLibrary.VSize` (- (`SceneComponent.K2_GetComponentLocation` (`/DynamicalSystems/Blueprints/BP_GravityCurve.DefaultSceneRoot` _gravitycurve)) (`SceneComponent.K2_GetComponentLocation` (`/DynamicalSystems/FullBodyIK/Blueprints/IK_Pawn.DefaultSceneRoot` (`self.IK_Pawn`))))) (`SphereComponent.GetScaledSphereRadius` (`/DynamicalSystems/Blueprints/BP_GravityCurve.SphereCollision` _gravitycurve))))))))))
      (:`then_6`
        (if (or (`self.GripLockedL`) (`self.GripLockedR`))
          (set `self.Gravity` 0.0001)))
      (:`then_7`
        (`self.SetViewTargetWithBlend` (`self.IK_Camera`))))))

(event `UpdateFromState`
  (params (delta :type "Float (double-precision)"))
  (bind (_asavatar_state _success) (`self.GetState`))
  (if _success
    (bind _asik_pawn_slim (cast `/DynamicalSystems/FullBodyIK/Blueprints/IK_Pawn_SLIM` (`self.IK_Pawn`)))
    (`/DynamicalSystems/State/AvatarState.SetObjectToAvatar` _asavatar_state null null (`/DynamicalSystems/FullBodyIK/Blueprints/IK_Pawn_SLIM.HMDCamera` _asik_pawn_slim) null false delta (`/DynamicalSystems/FullBodyIK/Blueprints/IK_Pawn_SLIM.Origin` _asik_pawn_slim))))

(fn `GetState`
  (returns (`AsAvatar State` :type "/DynamicalSystems/State/AvatarState Object Reference") (Success :type Boolean))
  (bind _asavatar_state (cast `/DynamicalSystems/State/AvatarState` (`self.PlayerState`))
    (:`then`
      _)
    (:`CastFailed`
      _))
  (return _asavatar_state (`KismetSystemLibrary.IsValid` _asavatar_state)))

(fn `UserConstructionScript`
  (`parent.UserConstructionScript`))

(fn `Validation`
  (returns (IsValid :type Boolean))
  (bind _ik_pawn (`self.IK_Pawn`))
  (bind _ik_pawn_2 (`self.IK_Pawn`))
  (`|ExecutionSequence`
    (:`then_0`
      (`/Engine/EditorBlueprintResources/StandardMacros.IsValid` (`self.IK_Pawn`)
        (:`Is Not Valid`
          (bind _asik_pawn (cast `/DynamicalSystems/FullBodyIK/Blueprints/IK_Pawn` (`self.K2_GetPawn`))
            (:`then`
              (bind _output_get (set `self.IK_Pawn` _asik_pawn))
              (`self.SetOwner` _output_get self))
            (:`CastFailed`
              (return false))))))
    (:`then_1`
      (`/Engine/EditorBlueprintResources/StandardMacros.IsValid` (`self.IK_Camera`)
        (:`Is Not Valid`
          (`/Engine/EditorBlueprintResources/StandardMacros.IsValid` _ik_pawn
            (:`Is Valid`
              (bind _returnvalue (`|SpawnActorFromClass` "/DynamicalSystems/FullBodyIK/Blueprints/IK_Camera.IK_Camera_C" (`SceneComponent.K2_GetComponentToWorld` (`/DynamicalSystems/FullBodyIK/Blueprints/IK_Pawn.DefaultSceneRoot` _ik_pawn)) "AlwaysSpawn" "OverrideRootScale" _ik_pawn null))
              (bind _output_get_2 (set `self.IK_Camera` _returnvalue))
              (`self.SetOwner` (`ChildActorComponent.ChildActor` (`/DynamicalSystems/FullBodyIK/Blueprints/IK_Pawn.ChildHMD` (`self.IK_Pawn`))) _output_get_2)
              (`self.SetViewTargetWithBlend` self (`self.IK_Pawn`) 0.0 "VTBlend_Linear" 0.0 false)
              (`|ExecutionSequence`
                (:`then_0`
                  (bind _asik_motion_controller (cast `/DynamicalSystems/FullBodyIK/Blueprints/IK_MotionController` (`ChildActorComponent.ChildActor` (`/DynamicalSystems/FullBodyIK/Blueprints/IK_Pawn.ChildMotionControllerL` _ik_pawn_2)))
                    (:`then`
                      (set `self.IK_MotionControllerL` _asik_motion_controller))
                    (:`CastFailed`
                      (return false))))
                (:`then_1`
                  (bind _asik_motion_controller_2 (cast `/DynamicalSystems/FullBodyIK/Blueprints/IK_MotionController` (`ChildActorComponent.ChildActor` (`/DynamicalSystems/FullBodyIK/Blueprints/IK_Pawn.ChildMotionControllerR` _ik_pawn_2)))
                    (:`then`
                      (set `self.IK_MotionControllerR` _asik_motion_controller_2))
                    (:`CastFailed`
                      (return false))))))
            (:`Is Not Valid`
              (return false))))))
    (:`then_3`
      (return true))))