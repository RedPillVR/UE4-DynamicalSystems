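; VR player controller for the full-body IK avatar, spawning and possessing an IK_Pawn at the PlayerStart with a separate IK_Camera as view target.
; Each tick it applies floor-trace following, stick locomotion and grip-latch climbing with inertia and distance-curve gravity.
; It then copies headset and controller transforms to the pawn and NetAvatar for networking.
; It also handles teleporting, height calibration, trigger hand-grip values and movement disabling for DJ mode.
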(event `InputAxisKey|MotionController_Left_TriggerAxis`
  (params (AxisValue :type "Float (single-precision)"))
  (bind _ik_pawn (`self.IK_Pawn`))
  (`/Engine/EditorBlueprintResources/StandardMacros.IsValid` _ik_pawn
    (:`Is Valid`
      (set `/DynamicalSystems/FullBodyIK/Characters/Mannequin/IK_Character.LeftHandGripping` AxisValue (`/DynamicalSystems/FullBodyIK/Blueprints/IK_Pawn.Character` _ik_pawn)))))

(event `InputAxisKey|MotionController_Right_TriggerAxis`
  (params (AxisValue :type "Float (single-precision)"))
  (bind _ik_pawn (`self.IK_Pawn`))
  (`/Engine/EditorBlueprintResources/StandardMacros.IsValid` _ik_pawn
    (:`Is Valid`
      (set `/DynamicalSystems/FullBodyIK/Characters/Mannequin/IK_Character.RightHandGripping` AxisValue (`/DynamicalSystems/FullBodyIK/Blueprints/IK_Pawn.Character` _ik_pawn)))))

(event `self.ReceiveBeginPlay`
  (bind _ik_camera (`self.IK_Camera`))
  (bind _ik_pawn (`self.IK_Pawn`))
  (`|ExecutionSequence`
    (:`then_0`
      (`HeadMountedDisplayFunctionLibrary.SetTrackingOrigin` "Floor"))
    (:`then_1`
      (bind _outactors (`GameplayStatics.GetAllActorsOfClass` "/Script/DynamicalSystems.NetClient"))
      (bind _output (`/DynamicalSystems/FullBodyIK/Blueprints/IK_MacroLibrary.Validated Get (A copy)` _outactors)
        (:`Exists`
          (bind _output_get (set `NetAvatar.NetClient` _output (`self.NetAvatar`)))
          (set `self.Net Client` _output_get))))
    (:`then_2`
      (bind _outactors_2 (`GameplayStatics.GetAllActorsOfClass` "/Script/Engine.PlayerStart"))
      (bind _output_2 (`/DynamicalSystems/FullBodyIK/Blueprints/IK_MacroLibrary.Validated Get (A copy)` _outactors_2)
        (:`Exists`
          (`|ExecutionSequence`
            (:`then_0`
              (bind _returnvalue (`|SpawnActorFromClass` "/DynamicalSystems/FullBodyIK/Blueprints/IK_Pawn.IK_Pawn_C" (`KismetMathLibrary.ComposeTransforms` (`KismetMathLibrary.MakeTransform` (0.0 0.0 100.0) (struct :`Yaw` -90.0)) (`self.GetTransform` _output_2)) "AlwaysSpawn" "OverrideRootScale" self null))
              (bind _output_get_2 (set `self.IK_Pawn` _returnvalue))
              (set `/DynamicalSystems/FullBodyIK/Blueprints/IK_Pawn.Player` self _output_get_2)
              (bind _returnvalue_2 (`|SpawnActorFromClass` "/DynamicalSystems/FullBodyIK/Blueprints/IK_Camera.IK_Camera_C" (`SceneComponent.K2_GetComponentToWorld` (`/DynamicalSystems/FullBodyIK/Blueprints/IK_Pawn.DefaultSceneRoot` _output_get_2)) "AlwaysSpawn" "OverrideRootScale" null null))
              (set `self.IK_Camera` _returnvalue_2)
              (`self.SetOwner` (`ChildActorComponent.ChildActor` (`/DynamicalSystems/FullBodyIK/Blueprints/IK_Pawn.ChildHMD` (`self.IK_Pawn`))) _ik_camera)
              (`self.Possess` self (`self.IK_Pawn`))
              (`self.SetViewTargetWithBlend` self _ik_camera 0.0 "VTBlend_Linear" 0.0 false)
              (`|ExecutionSequence`
                (:`then_0`
                  (bind _asik_motion_controller (cast `/DynamicalSystems/FullBodyIK/Blueprints/IK_MotionController` (`ChildActorComponent.ChildActor` (`/DynamicalSystems/FullBodyIK/Blueprints/IK_Pawn.ChildMotionControllerL` _ik_pawn))))
                  (set `self.IK_MotionControllerL` _asik_motion_controller))
                (:`then_1`
                  (bind _asik_motion_controller_2 (cast `/DynamicalSystems/FullBodyIK/Blueprints/IK_MotionController` (`ChildActorComponent.ChildActor` (`/DynamicalSystems/FullBodyIK/Blueprints/IK_Pawn.ChildMotionControllerR` _ik_pawn))))
                  (set `self.IK_MotionControllerR` _asik_motion_controller_2))))))))
    (:`then_3`
      (bind _outactors_3 (`GameplayStatics.GetAllActorsOfClass` "/DynamicalSystems/Blueprints/BP_GravityCurve.BP_GravityCurve_C"))
      (bind _output_3 (`/DynamicalSystems/FullBodyIK/Blueprints/IK_MacroLibrary.Validated Get (A copy)` _outactors_3)
        (:`Exists`
          (set `self.GravityCurve` _output_3))))))

(event `self.ReceiveTick`
  (params (DeltaSeconds :type "Float (single-precision)"))
  (bind _returnvalue (`KismetMathLibrary.MakeVector` 0.0 0.0 1.0))
  (bind _ik_pawn (`self.IK_Pawn`))
  (bind _netavatar (`self.NetAvatar`))
  (bind _netavatar_2 (`self.NetAvatar`))
  (bind _netavatar_3 (`self.NetAvatar`))
  (bind _netavatar_4 (`self.NetAvatar`))
  (bind _ik_pawn_2 (`self.IK_Pawn`))
  (bind _defaultsceneroot (`/DynamicalSystems/FullBodyIK/Blueprints/IK_Pawn.DefaultSceneRoot` (`self.IK_Pawn`)))
  (bind _defaultsceneroot_2 (`/DynamicalSystems/FullBodyIK/Blueprints/IK_Pawn.DefaultSceneRoot` (`self.IK_Pawn`)))
  (bind _returnvalue_2 (`SceneComponent.K2_GetComponentToWorld` (`/DynamicalSystems/FullBodyIK/Blueprints/IK_Camera.Camera` (`self.IK_Camera`))))
  (bind (_returnvalue_location _returnvalue_rotation) (`KismetMathLibrary.BreakTransform` (`SceneComponent.K2_GetComponentToWorld` (`/DynamicalSystems/FullBodyIK/Blueprints/IK_Pawn.DefaultSceneRoot` (`self.IK_Pawn`)))))
  (bind _returnvalue_3 (`KismetMathLibrary.ComposeTransforms` (`SceneComponent.GetRelativeTransform` (`self.MotionControllerR`)) (`SceneComponent.K2_GetComponentToWorld` (`/DynamicalSystems/FullBodyIK/Blueprints/IK_Camera.VROrigin` (`self.IK_Camera`)))))
  (bind _returnvalue_4 (`KismetMathLibrary.ComposeTransforms` (`SceneComponent.GetRelativeTransform` (`self.MotionControllerL`)) (`SceneComponent.K2_GetComponentToWorld` (`/DynamicalSystems/FullBodyIK/Blueprints/IK_Camera.VROrigin` (`self.IK_Camera`)))))
  (`/Engine/EditorBlueprintResources/StandardMacros.IsValid` _ik_pawn
    (:`Is Valid`
      (`|ExecutionSequence`
        (:`then_0`
          (`self.FloorNav` DeltaSeconds))
        (:`then_1`
          (`self.Latch` DeltaSeconds))
        (:`then_2`
          ;[1 1 1] Motion Controlled Locomotion
          (`SceneComponent.K2_SetWorldLocation` (`/DynamicalSystems/FullBodyIK/Blueprints/IK_Camera.DefaultSceneRoot` (`self.IK_Camera`)) (+ (+ (`SceneComponent.K2_GetComponentLocation` (`/DynamicalSystems/FullBodyIK/Blueprints/IK_Camera.DefaultSceneRoot` (`self.IK_Camera`))) (+ (* (`SceneComponent.GetRightVector` _defaultsceneroot_2) (* DeltaSeconds (* (* (* (`self.GetInputAxisValue`) 1.0) -150.0) (`KismetMathLibrary.Conv_BoolToDouble` (`self.MovementAllowed`))))) (* (`SceneComponent.GetForwardVector` _defaultsceneroot_2) 0.0))) (/ (+ (`self.GripLockedOffsetL`) (`self.GripLockedOffsetR`)) 2.0)) false false)
          (`SceneComponent.K2_SetWorldLocation` _defaultsceneroot (+ (* _returnvalue (`KismetMathLibrary.Dot_VectorVector` (* (`self.Thrust`) DeltaSeconds) _returnvalue)) (`SceneComponent.K2_GetComponentLocation` _defaultsceneroot) (/ (+ (`self.GripLockedOffsetL`) (`self.GripLockedOffsetR`)) 2.0)) false false))
        (:`then_3`
          (`SceneComponent.K2_SetWorldTransform` (`/DynamicalSystems/FullBodyIK/Blueprints/IK_Pawn.ChildMotionControllerL` (`self.IK_Pawn`)) _returnvalue_4 false false)
          (`SceneComponent.K2_SetWorldTransform` (`/DynamicalSystems/FullBodyIK/Blueprints/IK_Pawn.ChildMotionControllerR` (`self.IK_Pawn`)) _returnvalue_3 false false)
          (`SceneComponent.K2_SetWorldTransform` (`/DynamicalSystems/FullBodyIK/Blueprints/IK_Pawn.ChildHMD` (`self.IK_Pawn`)) _returnvalue_2 false false))
        (:`then_4`
          (set `NetAvatar.LocationHandL` (.location _returnvalue_4) _netavatar_3)
          (set `NetAvatar.RotationHandL` (.rotation _returnvalue_4) _netavatar_3)
          (set `NetAvatar.LocationHandR` (.location _returnvalue_3) _netavatar_4)
          (set `NetAvatar.RotationHandR` (.rotation _returnvalue_3) _netavatar_4)
          (set `NetAvatar.LocationHMD` (.location _returnvalue_2) _netavatar_2)
          (set `NetAvatar.RotationHMD` (.rotation _returnvalue_2) _netavatar_2)
          (set `NetAvatar.Location` _returnvalue_location _netavatar)
          (set `NetAvatar.Rotation` _returnvalue_rotation _netavatar)
          (set `NetAvatar.Floor` (`/DynamicalSystems/FullBodyIK/Blueprints/IK_Pawn.Floor` _ik_pawn_2) _netavatar)
          (set `NetAvatar.Height` (`/DynamicalSystems/FullBodyIK/Blueprints/IK_Pawn.Height` _ik_pawn_2) _netavatar))
        (:`then_5`
          (`/DynamicalSystems/FullBodyIK/Blueprints/IK_Pawn.SetBodyColor` _ik_pawn (`KismetMathLibrary.HSVToRGB` (* (/ (`KismetMathLibrary.Conv_IntToDouble` (mod (`NetAvatar.NetID` (`self.NetAvatar`)) 7)) 7.0) 360.0) 0.7 0.5)))))))

(event `InputAction|ViveTouchpadFace_L_Forward`
  (params (Key :type "Key Structure"))
  ;[1 1 1] KeyPress Gate
  (:`Pressed`
    (set `self.ForwardPress` 1.0 :!label _label))
  (:`Released`
    (set `self.ForwardPress` 0.0 :!label _label_2)))

(event `InputAction|ViveTouchpadFace_L_Back`
  (params (Key :type "Key Structure"))
  ;[1 1 1] KeyPress Gate
  (:`Pressed`
    (goto _label))
  (:`Released`
    (goto _label_2)))

(event `InputAction|CalibrateHeight`
  (params (Key :type "Key Structure")))

(event `Key|MotionController_Left_Shoulder`
  (params (Key :type "Key Structure"))
  ;[0 0 0] Calibrate Height on Controller until keyboard shows up in builds correctly.
  (:`Pressed`
    (`self.CalibrateHeight` :!label _label_3)))

(event `Key|MotionController_Right_Shoulder`
  (params (Key :type "Key Structure"))
  ;[0 0 0] Calibrate Height on Controller until keyboard shows up in builds correctly.
  (:`Pressed`
    (goto _label_3)))

(event `Key|MotionController_Right_FaceButton2`
  (params (Key :type "Key Structure"))
  ;[0 0 0] Calibrate Height on Controller until keyboard shows up in builds correctly.
  (:`Pressed`
    (if (`|EnumEquality` (`/DynamicalSystems/FullBodyIK/Blueprints/IK_Pawn.DeviceList` (`self.IK_Pawn`)) "NewEnumerator0")
      (goto _label_3))))

(event `InputAction|ToggleGravity`
  (params (Key :type "Key Structure")))

(fn `CalibrateHeight`
  (bind (_returnvalue_location _returnvalue_rotation) (`KismetMathLibrary.BreakTransform` (`SceneComponent.K2_GetComponentToWorld` (`/DynamicalSystems/FullBodyIK/Blueprints/IK_Camera.Camera` (`self.IK_Camera`)))))
  (`/Engine/EditorBlueprintResources/StandardMacros.IsValid` (`self.IK_Pawn`)
    (:`Is Valid`
      (bind _output_get (set `/DynamicalSystems/FullBodyIK/Blueprints/IK_Pawn.Height` (`KismetMathLibrary.FMax` (- (.z (.location (`SceneComponent.K2_GetComponentToWorld` (`/DynamicalSystems/FullBodyIK/Blueprints/IK_Camera.Camera` (`self.IK_Camera`))))) (`/DynamicalSystems/FullBodyIK/Blueprints/IK_Pawn.Floor` (`self.IK_Pawn`)))) (`self.IK_Pawn`)))
      (`KismetSystemLibrary.DrawDebugString` (+ _returnvalue_location (* (`KismetMathLibrary.GetForwardVector` _returnvalue_rotation) 100.0)) (`KismetTextLibrary.Conv_TextToString` (`|FormatText` "Calibrate Height: {Float}" _output_get)) null (struct :`R` 1.0 :`G` 0.535105 :`A` 1.0) 3.0))))

(fn `FloorNav`
  (params (DeltaTime :type "Float (double-precision)"))
  (locals (HeadOffset :type "Float (double-precision)" :default 0.0))
  (bind _defaultsceneroot (`/DynamicalSystems/FullBodyIK/Blueprints/IK_Camera.DefaultSceneRoot` (`self.IK_Camera`)))
  (bind _returnvalue (`SceneComponent.K2_GetComponentLocation` (`/DynamicalSystems/FullBodyIK/Blueprints/IK_Pawn.DefaultSceneRoot` (`self.IK_Pawn`))))
  (bind (_returnvalue_x _returnvalue_y _returnvalue_z) (`KismetMathLibrary.BreakVector` (`SceneComponent.K2_GetComponentLocation` (`/DynamicalSystems/FullBodyIK/Blueprints/IK_Camera.DefaultSceneRoot` (`self.IK_Camera`)))))
  (bind (_returnvalue_x_2 _returnvalue_y_2 _returnvalue_z_2) (`KismetMathLibrary.BreakVector` (`SceneComponent.K2_GetComponentLocation` (`/DynamicalSystems/FullBodyIK/Blueprints/IK_Pawn.DefaultSceneRoot` (`self.IK_Pawn`)))))
  (bind (_returnvalue_x_3 _returnvalue_y_3) (`KismetMathLibrary.BreakVector` (`SceneComponent.K2_GetComponentLocation` _defaultsceneroot)))
  (bind _x (.x (`SceneComponent.K2_GetComponentLocation` (`/DynamicalSystems/FullBodyIK/Blueprints/IK_Pawn.DefaultSceneRoot` (`self.IK_Pawn`)))))
  (bind _y (.y (`SceneComponent.K2_GetComponentLocation` (`/DynamicalSystems/FullBodyIK/Blueprints/IK_Pawn.DefaultSceneRoot` (`self.IK_Pawn`)))))
  (bind _z (.z (`SceneComponent.K2_GetComponentLocation` (`/DynamicalSystems/FullBodyIK/Blueprints/IK_Pawn.DefaultSceneRoot` (`self.IK_Pawn`)))))
  (set `local.HeadOffset` (- _returnvalue_z _z))
  (bind (_outhit _returnvalue_2) (`KismetSystemLibrary.LineTraceSingleForObjects` (`KismetMathLibrary.MakeVector` _x _y (+ _z 100.0)) (`KismetMathLibrary.MakeVector` _x _y (+ _z -20000.0)) (`|MakeArray` "ObjectTypeQuery1" "ObjectTypeQuery14" "ObjectTypeQuery10" :!type "EObjectTypeQuery Enum") false (`|MakeArray` (`self.IK_Pawn`) :!type "Actor Object Reference")))
  (if _returnvalue_2
    (bind (_bblockinghit _binitialoverlap _time _distance _location _impactpoint _normal) (`GameplayStatics.BreakHitResult` _outhit))
    (`SceneComponent.K2_SetWorldLocation` (`/DynamicalSystems/FullBodyIK/Blueprints/IK_Pawn.DefaultSceneRoot` (`self.IK_Pawn`)) (`KismetMathLibrary.VInterpTo` _returnvalue _location DeltaTime (`KismetMathLibrary.MapRangeClamped` (.z (- _location _returnvalue)) 50.0 -50.0 (* 1.0 20.0) (* (`self.Gravity`) 1.0))) false false)
    (bind _output_get (set `/DynamicalSystems/FullBodyIK/Blueprints/IK_Pawn.Floor` (.z _location) (`self.IK_Pawn`)))
    (`SceneComponent.K2_SetWorldLocation` _defaultsceneroot (`KismetMathLibrary.MakeVector` _returnvalue_x_3 _returnvalue_y_3 (+ (`local.HeadOffset`) _returnvalue_z_2)) false false)))

(fn `GetComponentsFor`
  (params (Gear :type Byte))
  (returns (NewParam1 :type "SceneComponent Object Reference"))
  (bind _asik_pawn (cast `/DynamicalSystems/FullBodyIK/Blueprints/IK_Pawn` (`self.K2_GetPawn`))
    (:`then`
      (switch `/DynamicalSystems/Interfaces/VRGearRequestType` (cast `/DynamicalSystems/Interfaces/VRGearRequestType` Gear)
        (:`NewEnumerator0`
          (return (`/DynamicalSystems/FullBodyIK/Blueprints/IK_Pawn.ChildHMD` _asik_pawn)))
        (:`NewEnumerator1`
          (return (`/DynamicalSystems/FullBodyIK/Blueprints/IK_Pawn.ChildMotionControllerL` _asik_pawn)))
        (:`NewEnumerator2`
          (return (`/DynamicalSystems/FullBodyIK/Blueprints/IK_Pawn.ChildMotionControllerR` _asik_pawn)))))
    (:`CastFailed`
      (return null))))

(fn `GetWSTransformFor`
  (params (RequestType :type "/DynamicalSystems/Interfaces/VRGearRequestType Enum" :default "NewEnumerator0"))
  (returns (WorldSpaceTransform :type "Transform Structure"))
  (bind _newparam1 (`self.GetComponentsFor` RequestType))
  (return (`SceneComponent.K2_GetComponentToWorld` _newparam1)))

(fn `Latch`
  (params (DeltaTime :type "Float (double-precision)"))
  (bind _gravitycurve (`self.GravityCurve`))
  (bind _returnvalue (`SceneComponent.K2_GetComponentLocation` (`/DynamicalSystems/FullBodyIK/Blueprints/IK_MotionController.OVSphere` (`self.IK_MotionControllerR`))))
  (bind _returnvalue_2 (`SceneComponent.K2_GetComponentLocation` (`/DynamicalSystems/FullBodyIK/Blueprints/IK_MotionController.OVSphere` (`self.IK_MotionControllerL`))))
  (`|ExecutionSequence`
    (:`then_0`
      (set `self.GripLockedOffsetR` (`KismetMathLibrary.VLerp` (`self.GripLockedOffsetR`) (0.0 0.0 0.0) (* DeltaTime 0.5))))
    (:`then_1`
      (set `self.GripLockedOffsetL` (`KismetMathLibrary.VLerp` (`self.GripLockedOffsetL`) (0.0 0.0 0.0) (* DeltaTime 0.5))))
    (:`then_2`
      (if (and (> (`self.GetInputAxisValue`) 0.5) (`/DynamicalSystems/FullBodyIK/Blueprints/IK_MotionController.IsOverlapping` (`self.IK_MotionControllerL`)))
        (if (not (`self.GripLockedL`))
          (set `self.GripLockedLocationL` _returnvalue_2)
          (set `self.GripLockedL` true)
          (set `self.GripLockedOffsetL` (0.0 0.0 0.0))
          (else
            (set `self.GripLockedOffsetL` (- (`self.GripLockedLocationL`) _returnvalue_2))))
        (elif (`self.GripLockedL`)
          (set `self.GripLockedL` false))))
    (:`then_3`
      (if (and (> (`self.GetInputAxisValue`) 0.5) (`/DynamicalSystems/FullBodyIK/Blueprints/IK_MotionController.IsOverlapping` (`self.IK_MotionControllerR`)))
        (if (not (`self.GripLockedR`))
          (set `self.GripLockedLocationR` _returnvalue)
          (set `self.GripLockedR` true)
          (set `self.GripLockedOffsetR` (0.0 0.0 0.0))
          (else
            (set `self.GripLockedOffsetR` (- (`self.GripLockedLocationR`) _returnvalue))))
        (elif (`self.GripLockedR`)
          (set `self.GripLockedR` false))))
    (:`then_4`
      (set `self.Gravity` (`KismetMathLibrary.Lerp` (`self.Gravity`) (`self.DefaultGravity`) (* DeltaTime 0.5))))
    (:`then_5`
      (`/Engine/EditorBlueprintResources/StandardMacros.IsValid` _gravitycurve
        (:`Is Valid`
          (bind _output_get (set `self.DefaultGravity` (- 1.0 (`CurveFloat.GetFloatValue` (`/DynamicalSystems/Blueprints/BP_GravityCurve.GravityCurve` (`self.GravityCurve`)) (/ (`KismetMathLibrary.VSize` (- (`SceneComponent.K2_GetComponentLocation` (`/DynamicalSystems/Blueprints/BP_GravityCurve.DefaultSceneRoot` _gravitycurve)) (`SceneComponent.K2_GetComponentLocation` (`/DynamicalSystems/FullBodyIK/Blueprints/IK_Pawn.DefaultSceneRoot` (`self.IK_Pawn`))))) (`SphereComponent.GetScaledSphereRadius` (`/DynamicalSystems/Blueprints/BP_GravityCurve.SphereCollision` _gravitycurve))))))))))
    (:`then_6`
      (if (or (`self.GripLockedL`) (`self.GripLockedR`))
        (set `self.Gravity` 0.0001)))))

(fn `MovementDisabler`
  (params (IsInDJMode :type Boolean))
  (returns (Success :type Boolean))
  (set `self.MovementAllowed` (not IsInDJMode))
  (return true))

(fn `TeleportTo`
  (params (Location :type "Vector Structure") (Rotation :type "Rotator Structure"))
  (locals (HeadOffset :type "Float (double-precision)") (CameraOffset :type "Vector Structure") (PawnOffset :type "Vector Structure") (SavedLocation :type "Vector Structure") (SavedRotation :type "Rotator Structure"))
  (bind _savedlocation (`local.SavedLocation`))
  (bind _returnvalue (`SceneComponent.K2_GetComponentLocation` (`/DynamicalSystems/FullBodyIK/Blueprints/IK_Camera.DefaultSceneRoot` (`self.IK_Camera`))))
  (bind (_returnvalue_x _returnvalue_y _returnvalue_z) (`KismetMathLibrary.BreakVector` (`SceneComponent.K2_GetComponentLocation` (`/DynamicalSystems/FullBodyIK/Blueprints/IK_Camera.DefaultSceneRoot` (`self.IK_Camera`)))))
  (bind (_returnvalue_x_2 _returnvalue_y_2) (`KismetMathLibrary.BreakVector` (- _returnvalue (`SceneComponent.K2_GetComponentLocation` (`/DynamicalSystems/FullBodyIK/Blueprints/IK_Pawn.DefaultSceneRoot` (`self.IK_Pawn`))))))
  (bind (_returnvalue_x_3 _returnvalue_y_3) (`KismetMathLibrary.BreakVector` (- _returnvalue (`SceneComponent.K2_GetComponentLocation` (`/DynamicalSystems/FullBodyIK/Blueprints/IK_Camera.Camera` (`self.IK_Camera`))))))
  ;[0 0 0] Store Local Vars
  (set `local.SavedLocation` Location)
  (set `local.SavedRotation` Rotation)
  ;[0 0 0] Camera & Pawn Offset
  (set `local.CameraOffset` (`KismetMathLibrary.MakeVector` _returnvalue_x_3 _returnvalue_y_3))
  (set `local.PawnOffset` (`KismetMathLibrary.MakeVector` _returnvalue_x_2 _returnvalue_y_2))
  ;[0 0 0] Head Offset
  (set `local.HeadOffset` (- _returnvalue_z (.z (`SceneComponent.K2_GetComponentLocation` (`/DynamicalSystems/FullBodyIK/Blueprints/IK_Pawn.DefaultSceneRoot` (`self.IK_Pawn`))))))
  ;[0 0 0] Check if sitting or standing
  (if true
    ;[0 0 0] Apply SEATED Camera & Pawn Location & Rotation
    (`SceneComponent.K2_SetWorldLocation` (`/DynamicalSystems/FullBodyIK/Blueprints/IK_Pawn.DefaultSceneRoot` (`self.IK_Pawn`)) (+ _savedlocation (`local.PawnOffset`)) false false)
    (`SceneComponent.K2_SetWorldLocation` (`/DynamicalSystems/FullBodyIK/Blueprints/IK_Camera.DefaultSceneRoot` (`self.IK_Camera`)) (`KismetMathLibrary.MakeVector` (.x (+ _savedlocation (`local.CameraOffset`))) (.y (+ _savedlocation (`local.CameraOffset`))) (+ (.z (+ _savedlocation (`local.CameraOffset`))) (`local.HeadOffset`))) false false)))

(fn `UserConstructionScript`)