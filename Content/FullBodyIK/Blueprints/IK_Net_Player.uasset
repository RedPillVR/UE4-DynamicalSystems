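; IK_Net_Player is a controller that drives a full-body IK pawn from networked VR avatar data.
; On BeginPlay it links its NetAvatar to the first NetClient, then spawns and possesses an IK_Pawn.
; Each Tick it interpolates the pawn's root, hands and HMD toward NetAvatar transforms, smoothing the root more slowly.
; It also copies height and floor, and derives body color from NetID in seven repeating hues.
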(event `self.ReceiveBeginPlay`
  (`|ExecutionSequence`
    (:`then_0`
      (bind _outactors (`GameplayStatics.GetAllActorsOfClass` "/Script/DynamicalSystems.NetClient"))
      (set `NetAvatar.NetClient` (`|GetArrayItem` _outactors) (`self.NetAvatar`)))
    (:`then_1`
      (bind _returnvalue (`|SpawnActorFromClass` "/DynamicalSystems/FullBodyIK/Blueprints/IK_Pawn.IK_Pawn_C" (`KismetMathLibrary.MakeTransform` (0.0 0.0 0.0)) "AlwaysSpawn" "OverrideRootScale" self null))
      (`|ExecutionSequence`
        (:`then_0`
          (`self.Possess` self _returnvalue))
        (:`then_1`
          (bind _output_get (set `self.IK_Pawn` _returnvalue))
          (set `/DynamicalSystems/FullBodyIK/Blueprints/IK_Pawn.Player` self _output_get))))))

(event `self.ReceiveTick`
  (params (DeltaSeconds :type "Float (single-precision)"))
  (bind _netavatar (`self.NetAvatar`))
  (bind _ik_pawn (`self.IK_Pawn`))
  (bind _netavatar_2 (`self.NetAvatar`))
  (bind _netavatar_3 (`self.NetAvatar`))
  (bind _netavatar_4 (`self.NetAvatar`))
  (bind _netavatar_5 (`self.NetAvatar`))
  (bind _defaultsceneroot (`/DynamicalSystems/FullBodyIK/Blueprints/IK_Pawn.DefaultSceneRoot` (`self.IK_Pawn`)))
  (bind (_returnvalue_location _returnvalue_rotation) (`KismetMathLibrary.BreakTransform` (`SceneComponent.K2_GetComponentToWorld` (`/DynamicalSystems/FullBodyIK/Blueprints/IK_Pawn.ChildHMD` (`self.IK_Pawn`)))))
  (bind (_returnvalue_location_2 _returnvalue_rotation_2) (`KismetMathLibrary.BreakTransform` (`SceneComponent.K2_GetComponentToWorld` (`/DynamicalSystems/FullBodyIK/Blueprints/IK_Pawn.ChildMotionControllerL` (`self.IK_Pawn`)))))
  (bind (_returnvalue_location_3 _returnvalue_rotation_3) (`KismetMathLibrary.BreakTransform` (`SceneComponent.K2_GetComponentToWorld` (`/DynamicalSystems/FullBodyIK/Blueprints/IK_Pawn.ChildMotionControllerR` (`self.IK_Pawn`)))))
  (`/Engine/EditorBlueprintResources/StandardMacros.IsValid` (`self.IK_Pawn`)
    (:`Is Valid`
      (`SceneComponent.K2_SetWorldTransform` (`/DynamicalSystems/FullBodyIK/Blueprints/IK_Pawn.DefaultSceneRoot` (`self.IK_Pawn`)) (`KismetMathLibrary.MakeTransform` (`KismetMathLibrary.VInterpTo` (`SceneComponent.K2_GetComponentLocation` _defaultsceneroot) (`NetAvatar.Location` _netavatar_5) DeltaSeconds 5.0) (`KismetMathLibrary.RInterpTo` (`SceneComponent.K2_GetComponentRotation` _defaultsceneroot) (`NetAvatar.Rotation` _netavatar_5) DeltaSeconds 5.0)) false false) ; pawn should set on event changed on itself
      (`SceneComponent.K2_SetWorldTransform` (`/DynamicalSystems/FullBodyIK/Blueprints/IK_Pawn.ChildMotionControllerL` (`self.IK_Pawn`)) (`KismetMathLibrary.MakeTransform` (`KismetMathLibrary.VInterpTo` _returnvalue_location_2 (`NetAvatar.LocationHandL` _netavatar_2) DeltaSeconds 10.0) (`KismetMathLibrary.RInterpTo` _returnvalue_rotation_2 (`NetAvatar.RotationHandL` _netavatar_2) DeltaSeconds 10.0)) false false)
      (`SceneComponent.K2_SetWorldTransform` (`/DynamicalSystems/FullBodyIK/Blueprints/IK_Pawn.ChildMotionControllerR` (`self.IK_Pawn`)) (`KismetMathLibrary.MakeTransform` (`KismetMathLibrary.VInterpTo` _returnvalue_location_3 (`NetAvatar.LocationHandR` _netavatar_4) DeltaSeconds 10.0) (`KismetMathLibrary.RInterpTo` _returnvalue_rotation_3 (`NetAvatar.RotationHandR` _netavatar_4) DeltaSeconds 10.0)) false false)
      (`SceneComponent.K2_SetWorldTransform` (`/DynamicalSystems/FullBodyIK/Blueprints/IK_Pawn.ChildHMD` (`self.IK_Pawn`)) (`KismetMathLibrary.MakeTransform` (`KismetMathLibrary.VInterpTo` _returnvalue_location (`NetAvatar.LocationHMD` _netavatar) DeltaSeconds 10.0) (`KismetMathLibrary.RInterpTo` _returnvalue_rotation (`NetAvatar.RotationHMD` _netavatar) DeltaSeconds 10.0)) false false)
      (`/DynamicalSystems/FullBodyIK/Blueprints/IK_Pawn.SetBodyColor` (`self.IK_Pawn`) (`KismetMathLibrary.HSVToRGB` (* (/ (`KismetMathLibrary.Conv_IntToDouble` (mod (`NetAvatar.NetID` (`self.NetAvatar`)) 7)) 7.0) 360.0) 0.7 0.5))
      (set `/DynamicalSystems/FullBodyIK/Blueprints/IK_Pawn.Height` (`NetAvatar.Height` _netavatar_3) _ik_pawn)
      (set `/DynamicalSystems/FullBodyIK/Blueprints/IK_Pawn.Floor` (`NetAvatar.Floor` _netavatar_3) _ik_pawn))))

(fn `UserConstructionScript`)