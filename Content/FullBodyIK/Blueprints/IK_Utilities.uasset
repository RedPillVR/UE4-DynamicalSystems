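; Utility function set for full-body IK avatars driven by an HMD and motion controllers.
; Avatar helpers fetch a row by index from a soft-referenced DataTable, caching the loaded table, then apply its mesh, anim class and materials.
; MeasureAvatar derives height and tracking-device offsets from mesh sockets.
; IKFootTrace converts a line trace at a socket into a scale-adjusted foot offset, and a debug helper draws segmented cubic Beziers with tangent arrows.
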(fn `DebugDrawCubicBezier`
  (params (Time :type "Float (double-precision)") (P0 :type "Vector Structure") (P1 :type "Vector Structure") (P2 :type "Vector Structure") (P3 :type "Vector Structure"))
  (bind _returnvalue (`KismetMathLibrary.Conv_IntToDouble` 30))
  (for _index (range 30)
    (`KismetSystemLibrary.DrawDebugLine` null (`DynamicalUtil.CubicBezier` (/ (`KismetMathLibrary.Conv_IntToDouble` _index) _returnvalue) P0 P1 P2 P3) (`DynamicalUtil.CubicBezier` (/ (`KismetMathLibrary.Conv_IntToDouble` (+ _index 1)) _returnvalue) P0 P1 P2 P3) (struct :`R` 1.0 :`G` 0.887345 :`A` 1.0) 0.0 1.0))
  (`|ExecutionSequence`
    (:`then_0`
      (`KismetSystemLibrary.DrawDebugArrow` null P0 P1 2.0 (struct :`R` 1.0 :`B` 0.654823 :`A` 1.0) 0.0 1.0))
    (:`then_1`
      (`KismetSystemLibrary.DrawDebugArrow` null P3 P2 2.0 (struct :`G` 0.573642 :`B` 1.0 :`A` 1.0) 0.0 1.0))))

(fn `GetAvatarFromTable`
  (params (Id :type Integer) (TableSoftRef :type "DataTable Soft Object Reference") (LoadedAvatarTable :type "DataTable Object Reference (by ref)"))
  (returns (Data :type "/DynamicalSystems/FullBodyIK/Characters/Mannequin/AvatarData Structure"))
  (`/Engine/EditorBlueprintResources/StandardMacros.IsValid` LoadedAvatarTable
    (:`Is Valid`
      (bind _outrownames (`DataTableFunctionLibrary.GetDataTableRowNames` LoadedAvatarTable :!label _label))
      (if (> (`KismetArrayLibrary.Array_Length` _outrownames) Id)
        (bind _returnvalue (`|GetDataTableRow` LoadedAvatarTable (`|GetArrayItem` _outrownames Id))
          (:`then`
            (`KismetSystemLibrary.PrintString` null "Found Avatar")
            (return _returnvalue))
          (:`RowNotFound`
            (`KismetSystemLibrary.PrintString` (`local.__WorldContext`) "row not found" false)))
        (else
          (`KismetSystemLibrary.PrintString` (`local.__WorldContext`) "No such index in table" false))))
    (:`Is Not Valid`
      (bind _asdata_table (cast `DataTable` (`AssetRegistryHelpers.GetAsset` (`AssetRegistryHelpers.CreateAssetData` (`|ConvertAsset` TableSoftRef))))
        (:`then`
          (`|VariableSetRef` LoadedAvatarTable _asdata_table)
          (goto _label))
        (:`CastFailed`
          (`KismetSystemLibrary.PrintString` (`local.__WorldContext`) "Not a table."))))))

(fn `IK_FootTrace`
  (params (SKMesh :type "SceneComponent Object Reference") (InSocketName :type Name) (Scale :type "Float (double-precision)") (TraceDistance :type "Float (double-precision)"))
  (returns (Offset :type "Float (double-precision)"))
  (bind _x (.x (`SceneComponent.GetSocketLocation` SKMesh InSocketName)))
  (bind _y (.y (`SceneComponent.GetSocketLocation` SKMesh InSocketName)))
  (bind _returnvalue (`KismetMathLibrary.MakeVector` _x _y (- (.z (`SceneComponent.K2_GetComponentLocation` SKMesh)) TraceDistance)))
  (bind _outhit (`KismetSystemLibrary.LineTraceSingle` SKMesh (`KismetMathLibrary.MakeVector` _x _y (+ _x TraceDistance)) _returnvalue "TraceTypeQuery3" false (`|MakeArray` (`ActorComponent.GetOwner` SKMesh)) "ForOneFrame"))
  (bind (_bblockinghit _binitialoverlap _time _distance _location) (`GameplayStatics.BreakHitResult` _outhit))
  (return (`KismetMathLibrary.SelectFloat` (/ (/ (`KismetMathLibrary.VSize` (- _returnvalue _location)) (.z (`SceneComponent.K2_GetComponentScale` SKMesh))) 2.0) 0.0 _bblockinghit)))

(fn `MeasureAvatar`
  (params (Mesh :type "SkeletalMeshComponent Object Reference (by ref)") (height :type "Float (double-precision) (by ref)") (HMDOffset :type "Transform Structure (by ref)") (LeftMotionControllerOffset :type "Transform Structure (by ref)") (RightMotionControllerOffset :type "Transform Structure (by ref)"))
  (returns (outheight :type "Float (double-precision)"))
  (locals (HMDSocketName :type Name :default "HMD") (FloorSocketName :type Name :default "Floor") (PelvisName :type Name :default "pelvis") (L_HandSocket :type Name :default "MC_L") (R_HandSocket :type Name :default "MC_R") (LHandBone :type Name :default "hand_l"))
  (bind _returnvalue (`KismetMathLibrary.VSize` (- (* (`SceneComponent.GetSocketLocation` Mesh (`local.HMDSocketName`)) (0.0 0.0 1.0)) (* (`SceneComponent.GetSocketLocation` Mesh (`local.FloorSocketName`)) (0.0 0.0 1.0)))))
  (`|ExecutionSequence`
    (:`then_0`
      (`|VariableSetRef` height _returnvalue)
      (`KismetSystemLibrary.PrintString` null (`KismetStringLibrary.Concat_StrStr` "height " (`KismetStringLibrary.Conv_DoubleToString` _returnvalue))))
    (:`then_1`
      (`|VariableSetRef` HMDOffset (`SceneComponent.GetSocketTransform` Mesh (`local.HMDSocketName`) "RTS_ParentBoneSpace")))
    (:`then_2`
      (`|VariableSetRef` LeftMotionControllerOffset (`SceneComponent.GetSocketTransform` Mesh (`local.L_HandSocket`) "RTS_ParentBoneSpace")))
    (:`then_3`
      (`|VariableSetRef` RightMotionControllerOffset (`SceneComponent.GetSocketTransform` Mesh (`local.R_HandSocket`) "RTS_ParentBoneSpace")))
    (:`then_4`
      (return _returnvalue))))

(fn `SetAvatar`
  (params (AvatarData :type "/DynamicalSystems/FullBodyIK/Characters/Mannequin/AvatarData Structure") (Target :type "SkeletalMeshComponent Object Reference (by ref)"))
  (bind (_mesh _animinstance) (break `/DynamicalSystems/FullBodyIK/Characters/Mannequin/AvatarData` AvatarData))
  (`SkinnedMeshComponent.SetSkinnedAssetAndUpdate` Target _mesh true)
  (`SkeletalMeshComponent.SetAnimInstanceClass` Target _animinstance)
  (for (_array_element _array_index) (`SkeletalMesh.Materials` _mesh)
    (`PrimitiveComponent.SetMaterial` Target _array_index (`.MaterialInterface` (break `SkeletalMaterial` _array_element)))
    (`KismetSystemLibrary.PrintText` (`local.__WorldContext`) (`|FormatText` "Avatar {name} w/ anim {anim}" (`KismetTextLibrary.Conv_StringToText` (`KismetSystemLibrary.GetObjectName` _mesh)) (`KismetTextLibrary.Conv_StringToText` (`KismetSystemLibrary.GetClassDisplayName` _animinstance))) false))
  (return))