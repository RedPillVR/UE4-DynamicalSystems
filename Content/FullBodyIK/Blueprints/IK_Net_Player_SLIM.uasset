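; Networked VR player controller that drives a full-body IK pawn from the avatar data in its AvatarState player state.
; It registers itself with that state, binds to its avatar updates and sets the pawn's body color.
; Height or floor changes go straight to the pawn.
; Any transform change updates root, HMD and both hands through VInterpTo/RInterpTo toward the NetAvatar values, driven by events instead of Tick.
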(event `self.ReceiveBeginPlay`
  (bind (_newparam _success) (`self.GetState`))
  (if _success
    (add `/DynamicalSystems/State/AvatarState.OnAvatarUpdate` _newparam (`|CreateDelegate` :!event `CustomEvent_0`))
    (`/DynamicalSystems/FullBodyIK/Blueprints/IK_Pawn.SetBodyColor` (`self.IK_Pawn`) (`/DynamicalSystems/State/AvatarState.AvatarColor` _newparam))))

(event `CustomEvent_0`
  (params (Floor :type "Float (double-precision)") (Height :type "Float (double-precision)") (Origin :type "Transform Structure") (Head :type "Transform Structure") (LHand :type "Transform Structure") (RHand :type "Transform Structure") (DimensionChanged :type "/DynamicalSystems/State/IK_Dimension Enum" :default "NewEnumerator2") (TransformChanged :type "/DynamicalSystems/State/IK_Transform Enum" :default "NewEnumerator4"))
  (bind _ik_pawn (`self.IK_Pawn`))
  (switch `/DynamicalSystems/State/IK_Transform` TransformChanged
    (:`NewEnumerator4`
      (switch `/DynamicalSystems/State/IK_Dimension` DimensionChanged
        (:`NewEnumerator0`
          (set `/DynamicalSystems/FullBodyIK/Blueprints/IK_Pawn.Height` Height _ik_pawn))
        (:`NewEnumerator1`
          (set `/DynamicalSystems/FullBodyIK/Blueprints/IK_Pawn.Floor` Floor _ik_pawn))))
    (:`NewEnumerator0`
      (`self.SetLocation` :!label _label)
      (`self.SetHMDTransform`)
      (`self.SetHand` "Left")
      (`self.SetHand` "Right"))
    (:`NewEnumerator1`
      (goto _label))
    (:`NewEnumerator2`
      (goto _label))
    (:`NewEnumerator3`
      (goto _label))))

(fn `GetState`
  (returns (NewParam :type "/DynamicalSystems/State/AvatarState Object Reference") (Success :type Boolean))
  (bind (_asavatar_state _bsuccess) (cast `/DynamicalSystems/State/AvatarState` (`self.PlayerState`) :!pure true))
  (return _asavatar_state _bsuccess))

(fn `SetHand`
  (params (Hand :type "EControllerHand Enum" :default "Left"))
  (locals (HandActor :type "ChildActorComponent Object Reference"))
  (bind _netavatar (`/DynamicalSystems/State/AvatarState.NetAvatar` (`self.GetState`)))
  (bind _netavatar_2 (`/DynamicalSystems/State/AvatarState.NetAvatar` (`self.GetState`)))
  (bind (_returnvalue_location _returnvalue_rotation) (`KismetMathLibrary.BreakTransform` (`SceneComponent.K2_GetComponentToWorld` (`/DynamicalSystems/FullBodyIK/Blueprints/IK_Pawn.ChildMotionControllerL` (`self.IK_Pawn`)))))
  (bind (_returnvalue_location_2 _returnvalue_rotation_2) (`KismetMathLibrary.BreakTransform` (`SceneComponent.K2_GetComponentToWorld` (`/DynamicalSystems/FullBodyIK/Blueprints/IK_Pawn.ChildMotionControllerR` (`self.IK_Pawn`)))))
  (switch `EControllerHand` Hand
    (:`Left`
      (`SceneComponent.K2_SetWorldTransform` (`/DynamicalSystems/FullBodyIK/Blueprints/IK_Pawn.ChildMotionControllerL` (`self.IK_Pawn`)) (`KismetMathLibrary.MakeTransform` (`KismetMathLibrary.VInterpTo` _returnvalue_location (`NetAvatar.LocationHandL` _netavatar_2) 0.0 10.0) (`KismetMathLibrary.RInterpTo` _returnvalue_rotation (`NetAvatar.RotationHandL` _netavatar_2) 0.0 10.0)) false false))
    (:`Right`
      (`SceneComponent.K2_SetWorldTransform` (`/DynamicalSystems/FullBodyIK/Blueprints/IK_Pawn.ChildMotionControllerR` (`self.IK_Pawn`)) (`KismetMathLibrary.MakeTransform` (`KismetMathLibrary.VInterpTo` _returnvalue_location_2 (`NetAvatar.LocationHandR` _netavatar) 0.0 10.0) (`KismetMathLibrary.RInterpTo` _returnvalue_rotation_2 (`NetAvatar.RotationHandR` _netavatar) 0.0 10.0)) false false))))

(fn `SetHMDTransform`
  (bind _netavatar (`/DynamicalSystems/State/AvatarState.NetAvatar` (`self.GetState`)))
  (bind (_returnvalue_location _returnvalue_rotation) (`KismetMathLibrary.BreakTransform` (`SceneComponent.K2_GetComponentToWorld` (`/DynamicalSystems/FullBodyIK/Blueprints/IK_Pawn.ChildHMD` (`self.IK_Pawn`)))))
  (`SceneComponent.K2_SetWorldTransform` (`/DynamicalSystems/FullBodyIK/Blueprints/IK_Pawn.ChildHMD` (`self.IK_Pawn`)) (`KismetMathLibrary.MakeTransform` (`KismetMathLibrary.VInterpTo` _returnvalue_location (`NetAvatar.LocationHMD` _netavatar) 0.0 10.0) (`KismetMathLibrary.RInterpTo` _returnvalue_rotation (`NetAvatar.RotationHMD` _netavatar) 0.0 10.0)) false false))

(fn `SetLocation`
  (bind _defaultsceneroot (`/DynamicalSystems/FullBodyIK/Blueprints/IK_Pawn.DefaultSceneRoot` (`self.IK_Pawn`)))
  (bind _netavatar (`/DynamicalSystems/State/AvatarState.NetAvatar` (`self.GetState`)))
  (`SceneComponent.K2_SetWorldTransform` (`/DynamicalSystems/FullBodyIK/Blueprints/IK_Pawn.DefaultSceneRoot` (`self.IK_Pawn`)) (`KismetMathLibrary.MakeTransform` (`KismetMathLibrary.VInterpTo` (`SceneComponent.K2_GetComponentLocation` _defaultsceneroot) (`NetAvatar.Location` _netavatar) 0.0 5.0) (`KismetMathLibrary.RInterpTo` (`SceneComponent.K2_GetComponentRotation` _defaultsceneroot) (`NetAvatar.Rotation` _netavatar) 0.0 5.0)) false false) ; pawn should set on event changed on itself
)

(fn `UserConstructionScript`
  (bind (_newparam _success) (`self.GetState`))
  (`parent.UserConstructionScript`)
  (if _success
    (set `/DynamicalSystems/State/AvatarState.Controller` self _newparam)))