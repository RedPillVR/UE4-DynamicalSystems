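; IK_Camera is a Blueprint in the FullBodyIK folder that manages the height of its VR origin for headset use.
; On BeginPlay it checks the HMD device name and, for SteamVR, calls SetVRHeightOffset with a zero offset.
; SetVRHeightOffset moves the VROrigin component to that relative Z height; a device-dependent height calculation is left unconnected, and Tick is empty.
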(event `self.ReceiveBeginPlay`
  (if (== (`HeadMountedDisplayFunctionLibrary.GetHMDDeviceName`) "SteamVR")
    (`self.SetVRHeightOffset` 0.0)))

(event `self.ReceiveTick`
  (params (DeltaSeconds :type "Float (single-precision)")))

(fn `SetVRHeightOffset`
  (params (`VR Offset` :type "Float (double-precision)"))
  (locals (DefaultOffset :type "Float (double-precision)"))
  (`SceneComponent.K2_SetRelativeLocation` (`self.VROrigin`) (`KismetMathLibrary.MakeVector` 0.0 0.0 `VR Offset`) false false))

(fn `UserConstructionScript`)