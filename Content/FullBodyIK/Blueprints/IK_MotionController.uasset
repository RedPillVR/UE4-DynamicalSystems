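; IK_MotionController is a Full Body IK motion controller Blueprint that tracks whether its overlap sphere is touching other components.
; OVSphere's begin and end overlap events add and remove the other component in the Overlaps collection.
; IsOverlapping reports true while that collection holds any entries.
; BeginPlay, Tick and the construction script are empty.
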(event `self.ReceiveBeginPlay`)

(event `self.OVSphere.OnComponentBeginOverlap`
  (params (OverlappedComponent :type "PrimitiveComponent Object Reference") (OtherActor :type "Actor Object Reference") (OtherComp :type "PrimitiveComponent Object Reference") (OtherBodyIndex :type Integer) (bFromSweep :type Boolean) (SweepResult :type "HitResult Structure (by ref)"))
  (if (== OverlappedComponent (`self.OVSphere`))
    (`BlueprintSetLibrary.Set_Add` (`self.Overlaps`) OtherComp)))

(event `self.OVSphere.OnComponentEndOverlap`
  (params (OverlappedComponent :type "PrimitiveComponent Object Reference") (OtherActor :type "Actor Object Reference") (OtherComp :type "PrimitiveComponent Object Reference") (OtherBodyIndex :type Integer))
  (`BlueprintSetLibrary.Set_Remove` (`self.Overlaps`) OtherComp))

(event `self.ReceiveTick`
  (params (DeltaSeconds :type "Float (single-precision)")))

(fn `IsOverlapping`
  (returns (Overlapping :type Boolean))
  (return (> (`BlueprintSetLibrary.Set_Length` (`self.Overlaps`)) 0)))

(fn `UserConstructionScript`)